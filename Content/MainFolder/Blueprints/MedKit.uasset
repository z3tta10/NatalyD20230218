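; MedKit is a pickup actor that heals the player character when they walk into its Box trigger.
; On overlap it casts to ThirdPersonCharacter and reads CurrentHP on that character's StatusAS.
; Below full health it adds a fixed amount capped at the maximum, destroys itself and prints a pickup message.
; At full health it stays in the world and prints that health is full.
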(event `self.Box.OnComponentBeginOverlap`
  (params (OverlappedComponent :type "PrimitiveComponent Object Reference") (OtherActor :type "Actor Object Reference") (OtherComp :type "PrimitiveComponent Object Reference") (OtherBodyIndex :type Integer) (bFromSweep :type Boolean) (SweepResult :type "HitResult Structure (by ref)"))
  (bind _asthird_person_character (cast `/Game/MainFolder/Blueprints/ThirdPersonCharacter` OtherActor))
  (bind _statusas (`/Game/MainFolder/Blueprints/ThirdPersonCharacter.StatusAS` _asthird_person_character))
  (if (>= (`/Game/MainFolder/Blueprints/StatusAS.CurrentHP` _statusas) 100.0)
    (`KismetSystemLibrary.PrintString` "Health is full")
    (else
      (set `/Game/MainFolder/Blueprints/StatusAS.CurrentHP` (`KismetMathLibrary.FMin` (+ (`/Game/MainFolder/Blueprints/StatusAS.CurrentHP` (`/Game/MainFolder/Blueprints/ThirdPersonCharacter.StatusAS` _asthird_person_character)) 25.0) 100.0) _statusas)
      (`self.K2_DestroyActor`)
      (`KismetSystemLibrary.PrintString` "You have found a MedKit"))))

(fn `UserConstructionScript`)