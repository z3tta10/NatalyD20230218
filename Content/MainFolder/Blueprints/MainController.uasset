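; Player controller that owns the main HUD widget, tracks the player character's health and handles game over and respawn.
; BeginPlay creates the widget and caches the possessed ThirdPersonCharacter.
; Tick pushes HP from the character's StatusAS to the widget and switches screens when life state changes, playing the game-over animation on death.
; Restart spawns and possesses a new character at the first PlayerStart found.
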(event `self.ReceiveBeginPlay`
  (`|ExecutionSequence`
    (:`then_0`
      (bind _returnvalue (`|CreateWidget` "/Game/MainFolder/UIX/MainWidget.MainWidget_C"))
      (set `self.MainWidget` _returnvalue)
      (`UserWidget.AddToViewport` (`self.MainWidget`) 0))
    (:`then_1`
      (bind _asthird_person_character (cast `/Game/MainFolder/Blueprints/ThirdPersonCharacter` (`self.K2_GetPawn`)))
      (set `self.MainPawn` _asthird_person_character))))

(event `self.ReceiveTick`
  (params (DeltaSeconds :type "Float (single-precision)"))
  (bind _statusas (`/Game/MainFolder/Blueprints/ThirdPersonCharacter.StatusAS` (`self.MainPawn`)))
  (`|ExecutionSequence`
    (:`then_0`
      ;[0.09237 0.8601 1] Update Health
      (`/Game/MainFolder/UIX/MainWidget.UpdateHealth` (`self.MainWidget`) (`/Game/MainFolder/Blueprints/StatusAS.CurrentHP` _statusas) (`/Game/MainFolder/Blueprints/StatusAS.MaxHP` _statusas)))
    (:`then_1`
      (if (`self.PlayerAlive`)
        ;[1 0.585 0.1354] Switch Screens
        (if (<= (`/Game/MainFolder/Blueprints/StatusAS.CurrentHP` (`/Game/MainFolder/Blueprints/ThirdPersonCharacter.StatusAS` (`self.MainPawn`))) 0.0)
          (set `self.PlayerAlive` false)
          (`/Game/MainFolder/UIX/MainWidget.SwitchScreen` (`self.MainWidget`) 1)
          (`/Game/MainFolder/UIX/MainWidget.PlayGameOverAnimation` (`self.MainWidget`)))
        (elif (> (`/Game/MainFolder/Blueprints/StatusAS.CurrentHP` (`/Game/MainFolder/Blueprints/ThirdPersonCharacter.StatusAS` (`self.MainPawn`))) 0.0)
          (set `self.PlayerAlive` true)
          (`/Game/MainFolder/UIX/MainWidget.SwitchScreen` (`self.MainWidget`) 0))))))

(event `Restart`
  ;[0.2825 1 0.5252] Restart, make new controlled pawn
  (bind _outactors (`GameplayStatics.GetAllActorsOfClass` "/Script/Engine.PlayerStart"))
  (bind _returnvalue (`|SpawnActorFromClass` "/Game/MainFolder/Blueprints/ThirdPersonCharacter.ThirdPersonCharacter_C" (`self.GetTransform` (`|GetArrayItem` _outactors)) "AlwaysSpawn" "OverrideRootScale" null null))
  (set `self.MainPawn` _returnvalue)
  (`self.UnPossess`)
  (`self.Possess` (`self.MainPawn`)))

(fn `UserConstructionScript`)